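; Blueprint that builds a blocky cube-grid terrain in its construction script, gated by a RenderInEditor flag.
; It loops over a square grid, setting each block's height from three summed sine-product waves with adjustable frequency and amplitude, rounded and scaled to block size.
; Blocks below a separation height go to a dirt instanced static mesh and the rest to a grass one, sharing one mesh with separate materials.
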(fn `UserConstructionScript`
  (bind _frequency3 (`self.Frequency3`))
  (bind _frequency2 (`self.Frequency2`))
  (bind _frequency1 (`self.Frequency1`))
  (bind _mesh (`self.Mesh`))
  (bind _block_size (`self.Block Size`))
  (bind _terrain_size (`self.Terrain Size`))
  (if (`self.Render in editor ?`)
    (`StaticMeshComponent.SetStaticMesh` (`self.DirtInstancedStaticMesh`) _mesh)
    (`StaticMeshComponent.SetStaticMesh` (`self.GrassInstancedStaticMesh`) _mesh)
    (`PrimitiveComponent.SetMaterial` (`self.GrassInstancedStaticMesh`) 0 (`self.Grass Material`))
    (`PrimitiveComponent.SetMaterial` (`self.DirtInstancedStaticMesh`) 0 (`self.Dirt Material`))
    (for _index (range (+ _terrain_size 1))
      (for _index_2 (range (+ _terrain_size 1))
        (bind _returnvalue (`KismetMathLibrary.Conv_VectorToTransform` (`KismetMathLibrary.MakeVector` (`KismetMathLibrary.Conv_IntToDouble` (* _index _block_size)) (`KismetMathLibrary.Conv_IntToDouble` (* _index_2 _block_size)) (`KismetMathLibrary.Conv_IntToDouble` (* (`KismetMathLibrary.Round` (+ (* (`KismetMathLibrary.DegSin` (* _index _frequency1)) (`KismetMathLibrary.DegSin` (* _index_2 _frequency1)) (`self.Height1`)) (* (`KismetMathLibrary.DegSin` (* _index _frequency2)) (`KismetMathLibrary.DegSin` (* _index_2 _frequency2)) (`self.Height2`)) (* (`KismetMathLibrary.DegSin` (* _index _frequency3)) (`KismetMathLibrary.DegSin` (* _index_2 _frequency3)) (`self.Height3`)))) (`self.Block Size`))))))
        (if (> (`self.Grass-Dirt Separation Height`) (.z (.location _returnvalue)))
          (`InstancedStaticMeshComponent.AddInstance` (`self.DirtInstancedStaticMesh`) _returnvalue false)
          (else
            (`InstancedStaticMeshComponent.AddInstance` (`self.GrassInstancedStaticMesh`) _returnvalue false)))))))